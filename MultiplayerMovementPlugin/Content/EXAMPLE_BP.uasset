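; Example character Blueprint that demonstrates a grapple hook built on a multiplayer movement component's replicated launch.
; The hook event sphere-traces along the follow camera's forward vector and, on a hit, launches the character upward.
; A short timer then launches it toward the hit location with velocity scaled by distance.
; An "All Nodes" section displays the component's other movement functions as unconnected nodes, alongside empty custom-movement events.
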(event `Example Grapple Hook`
  (bind _returnvalue (`self.K2_GetActorLocation`))
  ;[1 1 1] Trace to Find Where to Grapple
  (bind (_outhit _returnvalue_2) (`KismetSystemLibrary.SphereTraceSingle` _returnvalue (+ _returnvalue (* (`SceneComponent.GetForwardVector` (`self.FollowCamera`)) 10000.0)) 30.0 "TraceTypeQuery1" false (`|MakeArray` self :!type "Actor Object Reference") "ForDuration"))
  (if _returnvalue_2
    ;[1 1 1] Launch Up So the Character isn't on the ground
    (`MyCharacterMovementComponent.LaunchCharacterReplicated` (`self.GetMultiplayerMovementComponent`) (0.0 0.0 500.0) true true)
    ;[1 1 1] Timer To Let Character Launch Upwards Then Launch towards the Grapple Hook
    (bind _returnvalue_3 (`KismetSystemLibrary.K2_SetTimerDelegate` (delegate `Grapple To Location`) 0.2))
    (set `self.Grapple Handle` _returnvalue_3)))

(event `Grapple To Location`
  ;[1 1 1] Timer To Let Character Launch Upwards Then Launch towards the Grapple Hook
  (`MyCharacterMovementComponent.LaunchCharacterReplicated` (`self.GetMultiplayerMovementComponent`) (* (- (`.Location` (`GameplayStatics.BreakHitResult` (stale `Example Grapple Hook` _outhit))) (`self.K2_GetActorLocation`)) 2.5) false false))

(event `self.PhysNetCustom`
  (params (DeltaTime :type "Float (single-precision)") (Iterations :type Integer))
  ;[1 1 1] All Nodes
)

(event `self.OnMovementUpdatedCustom`
  (params (DeltaSeconds :type "Float (single-precision)") (OldLocation :type "Vector Structure (by ref)") (OldVelocity :type "Vector Structure (by ref)"))
  ;[1 1 1] All Nodes
)

(fn `UserConstructionScript`)